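; Player character Blueprint providing movement, look and a stamina-limited sprint.
; Movement follows control-rotation yaw, and the sprint input switches between run and walk speeds when enough stamina is available.
; Tick uses Delay nodes to pace stamina drain and regeneration to one-second steps, printing each new value.
; Empty stamina forces walking and holds regeneration for a configurable delay.
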(event `self.ReceiveBeginPlay`)

(event `self.ReceiveTick`
  (params (DeltaSeconds :type "Float (single-precision)"))
  ;[0 0 0] Sprint Stamina
  (`|ExecutionSequence`
    (:`then_0`
      (if (`self.isSprinting`)
        (`KismetSystemLibrary.Delay` 1.0)
        (`self.Stamina Drain`)
        (elif (`self.Stamina Depleted`)
          (`KismetSystemLibrary.Delay` (`self.Stamina Regen Delay`))
          (set `self.Stamina Depleted` false)
          (else
            (`KismetSystemLibrary.Delay` 1.0)
            (`self.Stamina Regen`)))))))

(event `InputAxis|Move Forward/Backward`
  (params (AxisValue :type "Float (single-precision)"))
  ;[0 0 0] Movement and Rotation
  (`self.AddMovementInput` (`self.Character Rotation`) AxisValue))

(event `InputAxis|Move Right/Left`
  (params (AxisValue :type "Float (single-precision)"))
  ;[0 0 0] Movement and Rotation
  (`self.AddMovementInput` (`.RightVector` (`self.Character Rotation`)) AxisValue))

(event `InputAxis|Look Up/Down`
  (params (AxisValue :type "Float (single-precision)"))
  ;[0 0 0] Movement and Rotation
  (`self.AddControllerPitchInput` AxisValue))

(event `InputAxis|Turn Right/Left`
  (params (AxisValue :type "Float (single-precision)"))
  ;[0 0 0] Movement and Rotation
  (`self.AddControllerYawInput` AxisValue))

(event `InputAction|Sprinting`
  (params (Key :type "Key Structure"))
  ;[0 0 0] Sprinting
  (:`Pressed`
    (if (>= (`self.Sprint Stamina`) (`self.Increase Stamina`))
      (set `self.isSprinting` true)
      (set `CharacterMovementComponent.MaxWalkSpeed` (`self.Run Speed`) (`self.CharacterMovement`))
      (else
        (set `self.isSprinting` false))))
  (:`Released`
    (set `CharacterMovementComponent.MaxWalkSpeed` (`self.Walk Speed`) (`self.CharacterMovement`))
    (set `self.isSprinting` false)))

(fn `Character Rotation`
  (returns (ForwardVector :type "Vector Structure") (RightVector :type "Vector Structure"))
  (bind _returnvalue (`KismetMathLibrary.MakeRotator` 0.0 0.0 (.yaw (`self.GetControlRotation`))))
  (return (`KismetMathLibrary.GetForwardVector` _returnvalue) (`KismetMathLibrary.GetRightVector` _returnvalue)))

(fn `Stamina Drain`
  (if (<= (`self.Sprint Stamina`) 0)
    (set `self.Stamina Depleted` true)
    (set `self.isSprinting` false)
    (set `CharacterMovementComponent.MaxWalkSpeed` (`self.Walk Speed`) (`self.CharacterMovement`))
    (else
      (bind _output_get (set `self.Sprint Stamina` (`KismetMathLibrary.Clamp` (- (`self.Sprint Stamina`) (`self.Decrease Stamina`)) 0 100)))
      (`KismetSystemLibrary.PrintString` (`KismetStringLibrary.Conv_IntToString` _output_get)))))

(fn `Stamina Regen`
  (if (< (`self.Sprint Stamina`) (`self.Max Sprint Stamina`))
    (bind _output_get (set `self.Sprint Stamina` (`KismetMathLibrary.Clamp` (+ (`self.Sprint Stamina`) (`self.Increase Stamina`)) 0 100)))
    (`KismetSystemLibrary.PrintString` (`KismetStringLibrary.Conv_IntToString` _output_get))))

(fn `UserConstructionScript`)